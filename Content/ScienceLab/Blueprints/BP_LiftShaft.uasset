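; BP_LiftShaft is a science lab lift call point that summons a lift when the player interacts with it.
; Each interaction sends a manual call to the linked lift, even when one is already on the way.
; A new call plays a click, notifies the linked door, and sets an on-the-way flag that clears after a fixed delay.
; While that flag is set, further presses only add a failure sound and message.
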(event EventOnInteract
  ;[0.125 0.125 0.125] No Lift Security
  (Default|ManualCall (Variables|Default|GetLikedLift))
  (if (Variables|Default|GetLiftOnTheWay)
    (Audio|PlaySound2D "/Engine/EditorSounds/Notifications/CompileFailed_Cue.CompileFailed_Cue" 1.0 1.0 0.0 0 0)
    (Development|PrintString "Lift Is allready on the way")
    (else
      (Variables|Default|SetLiftOnTheWay true)
      (Development|PrintString "Lift Called")
      (Audio|PlaySound2D "/Engine/VREditor/Sounds/UI/Click_on_Button_Cue.Click_on_Button_Cue" 1.0 1.0 0.0 0 0)
      (Default|LiftComming (Variables|Default|GetLinkedDoor))
      (Utilities|FlowControl|Delay 15.0)
      (Variables|Default|SetLiftOnTheWay false))))

(fn ConstructionScript)